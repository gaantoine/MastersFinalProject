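; NPC character that obeys coded sound-signal commands addressed to its ID tag, shown on front and rear child actors.
; Unprocessed signals are parsed by substring into follow, move, attack or cancel events for the AI controller's State Tree, with targets looked up through the puzzle manager.
; A hand-bone sphere trace deals melee damage.
; BPCDamageSystem handles health and death, which triggers ragdoll, list removal and destruction.
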(event `self.ReceiveBeginPlay`
  (bind _asidtag_front (cast `/Game/Blueprints/IDTagFront` (`ChildActorComponent.ChildActor` (`self.IDTagFront`))))
  (set `self.FrontID` _asidtag_front)
  (bind _asidtag_rear (cast `/Game/Blueprints/IDTagRear` (`ChildActorComponent.ChildActor` (`self.IDTagRear`))))
  (set `self.RearID` _asidtag_rear)
  (bind _output_get (set `self.IDNumber` (`/Game/Blueprints/IDTagFront.IDNumber` (`self.FrontID`))))
  (`/Game/Blueprints/IDTagRear.UpdateIDTagRear` (`self.RearID`) _output_get (`self.RearIDVisibility`))
  (`/Game/Blueprints/IDTagFront.UpdateIDTagFrontVisibility` (`self.FrontID`) (`self.FrontIDVisibility`))
  (bind _output_get_2 (set `self.NPC_AI_Controller` (`AIBlueprintHelperLibrary.GetAIController` self)))
  (bind _asai_npc (cast `/Game/AI/AI_NPC` _output_get_2))
  (set `self.StateTree` (`/Game/AI/AI_NPC.StateTreeAI` _asai_npc))
  (bind _returnvalue (`GameplayStatics.GetActorOfClass` "/Game/Blueprints/BP_PuzzleManager.BP_PuzzleManager_C"))
  (set `self.PuzzleManager` _returnvalue))

(event `/Game/Blueprints/BPI_Sound_Reaction.SoundReceived`
  (params (Signal :type "/Game/Blueprints/S_Signal Structure"))
  (bind (_receivedsignal_signalstring _receivedsignal_signalchain _receivedsignal_lowfrequencysignal _receivedsignal_impactpoint _receivedsignal_normal _receivedsignal_signalid) (break `/Game/Blueprints/S_Signal` (`self.ReceivedSignal`)))
  (bind (_receivedsignal_signalstring_2 _receivedsignal_signalchain_2 _receivedsignal_lowfrequencysignal_2 _receivedsignal_impactpoint_2 _receivedsignal_normal_2 _receivedsignal_signalid_2) (break `/Game/Blueprints/S_Signal` (`self.ReceivedSignal`)))
  (bind (_receivedsignal_signalstring_3 _receivedsignal_signalchain_3 _receivedsignal_lowfrequencysignal_3 _receivedsignal_impactpoint_3 _receivedsignal_normal_3 _receivedsignal_signalid_3) (break `/Game/Blueprints/S_Signal` (`self.ReceivedSignal`)))
  (if (`self.RespondsToSounds`)
    (bind _output_get (set `self.ReceivedSignal` Signal))
    (bind _output_get_2 (set `self.TransmissionString` (break `/Game/Blueprints/S_Signal` _output_get)))
    ; Check to see if the transmitted signal is meant for this actor
    (if (`KismetStringLibrary.EqualEqual_StrStr` (`self.IDNumber`) (`KismetStringLibrary.GetSubstring` _output_get_2 3 4))
      ; Check the length of the ProcessedSignals array.  If it is zero then we can pass the signal through without checking.  Otherwise we have to check the ReceivedSignal against entries in ProcessedSignals
      (if (== (`KismetArrayLibrary.Array_Length` (`self.ProcessedSignals`)) 0)
        ; If ReceivedSignal is the first signal ever received by this actor, add it to ProcessedSignals and process it
        (`KismetArrayLibrary.Array_AddUnique` (`self.ProcessedSignals`) _receivedsignal_signalid)
        (switch `string` (`KismetStringLibrary.GetSubstring` (`self.TransmissionString`) 0 3) :!label _label
          (:`FOL`
            (`KismetSystemLibrary.PrintString` "Confirmed Follow Comand Received" true true (struct :`G` 0.66 :`B` 1.0 :`A` 1.0) 10.0)
            (`StateTreeComponent.SendStateTreeEvent` (`self.StateTree`) (make `StateTreeEvent` (struct :`TagName` "Follow"))))
          (:`MOV`
            (`KismetSystemLibrary.PrintString` "Confirmed MoveTo Comand Received" true true (struct :`G` 0.66 :`B` 1.0 :`A` 1.0) 10.0)
            (for _array_element (`/Game/Blueprints/BP_PuzzleManager.DestinationActors` (`self.PuzzleManager`))
              (`/Engine/EditorBlueprintResources/StandardMacros.IsValid` _array_element
                (:`Is Valid`
                  (if (`KismetStringLibrary.EqualEqual_StrStr` (`/Game/Blueprints/BP_TargetDestination.IDNumber` _array_element) (`KismetStringLibrary.GetSubstring` (`self.TransmissionString`) 7 4))
                    (set `self.TargetDestination` (`/Game/Blueprints/BP_TargetDestination.DL_Position` _array_element))
                    (set `self.HasValidMoveToDestination` true)
                    (break)))))
            (if (`self.HasValidMoveToDestination`)
              (`StateTreeComponent.SendStateTreeEvent` (`self.StateTree`) (make `StateTreeEvent` (struct :`TagName` "MoveTo")))
              (set `self.HasValidMoveToDestination` false)))
          (:`ATK`
            (`KismetSystemLibrary.PrintString` "Confirmed Attack Comand Received" true true (struct :`G` 0.66 :`B` 1.0 :`A` 1.0) 10.0)
            (for _array_element_2 (`/Game/Blueprints/BP_PuzzleManager.DestinationActors` (`self.PuzzleManager`))
              (`/Engine/EditorBlueprintResources/StandardMacros.IsValid` _array_element_2
                (:`Is Valid`
                  (if (`KismetStringLibrary.EqualEqual_StrStr` (`/Game/Blueprints/BP_TargetDestination.IDNumber` _array_element_2) (`KismetStringLibrary.GetSubstring` (`self.TransmissionString`) 7 4))
                    (set `self.AttackTarget` _array_element_2)
                    (set `self.HasValidAttackTarget` true)
                    (break)))))
            (if (`self.HasValidAttackTarget`)
              (`StateTreeComponent.SendStateTreeEvent` (`self.StateTree`) (make `StateTreeEvent` (struct :`TagName` "Attack")))
              (set `self.HasValidAttackTarget` false)
              (else
                (for _array_element_3 (`/Game/Blueprints/BP_PuzzleManager.NPCActors` (`self.PuzzleManager`))
                  (`/Engine/EditorBlueprintResources/StandardMacros.IsValid` _array_element_3
                    (:`Is Valid`
                      (bind _idnumber (`/Game/AI/BP_NPC.IDNumber` _array_element_3))
                      (if (and (`KismetStringLibrary.NotEqual_StrStr` (`self.IDNumber`) _idnumber) (`KismetStringLibrary.EqualEqual_StrStr` _idnumber (`KismetStringLibrary.GetSubstring` (`self.TransmissionString`) 7 4)))
                        (set `self.AttackTarget` _array_element_3)
                        (set `self.HasValidAttackTarget` true)
                        (break)))))
                (if (`self.HasValidAttackTarget`)
                  (`StateTreeComponent.SendStateTreeEvent` (`self.StateTree`) (make `StateTreeEvent` (struct :`TagName` "Attack")))
                  (set `self.HasValidAttackTarget` false)))))
          (:`CAN`
            (`KismetSystemLibrary.PrintString` "Confirmed Cancel Comand Received" true true (struct :`G` 0.66 :`B` 1.0 :`A` 1.0) 10.0)
            (`StateTreeComponent.SendStateTreeEvent` (`self.StateTree`) (make `StateTreeEvent` (struct :`TagName` "Idle")))))
        (else
          ; If ReceivedSignal is not the first signal ever processed, its GUID must be compared against all previously received signal IDs to prevent duplicate activations
          (for _array_element_4 (`self.ProcessedSignals`)
            (if (== _array_element_4 _receivedsignal_signalid_2)
              (set `self.ReceivedSignalValid` false)
              (break)
              (else
                (set `self.ReceivedSignalValid` true))))
          ; If ReceivedSignal is confirmed to not be a duplicate, add its GUID to ProcessedSignals and continue with execution of logic
          (if (`self.ReceivedSignalValid`)
            (`KismetArrayLibrary.Array_AddUnique` (`self.ProcessedSignals`) _receivedsignal_signalid_3)
            (goto _label)))))))

(event `DealDamage`
  (bind _returnvalue_location (`KismetMathLibrary.BreakTransform` (`SkinnedMeshComponent.GetBoneTransform` (`self.Mesh`) "index_01_r" "RTS_World")))
  (bind _outhits (`KismetSystemLibrary.SphereTraceMultiForObjects` :`Start` _returnvalue_location :`End` _returnvalue_location :`Radius` 30.0 :`ObjectTypes` (`|MakeArray` "ObjectTypeQuery2" "ObjectTypeQuery3" "ObjectTypeQuery1" :!type "EObjectTypeQuery Enum") :`DrawDebugType` "ForDuration" :`DrawTime` 2.0))
  (for _array_element _outhits
    (bind (_bblockinghit _binitialoverlap _time _distance _location _impactpoint _normal _impactnormal _physmat _hitactor) (`GameplayStatics.BreakHitResult` _array_element))
    (if (not (`KismetArrayLibrary.Array_Contains` (`self.HitActors`) _hitactor))
      (message `/Game/Blueprints/BPI_Damageable.TakeDamage` _hitactor (make `/Game/Blueprints/S_DamageInfo` 50.0))
      (`KismetArrayLibrary.Array_AddUnique` (`self.HitActors`) _hitactor)))
  (`KismetArrayLibrary.Array_Clear` (`self.HitActors`)))

(event `OnDeath`
  (bind _mesh (`self.Mesh`))
  (`PrimitiveComponent.SetSimulatePhysics` _mesh true)
  (`PrimitiveComponent.SetCollisionEnabled` _mesh "QueryAndPhysics")
  (`/Game/Blueprints/BP_PuzzleManager.RemoveActorFromLists` (`self.PuzzleManager`) self)
  (`KismetSystemLibrary.Delay` 1.0)
  (`self.K2_DestroyActor`))

(event `OnDamageResponse`)

(fn `GetCurrentHealth`
  (returns (CurrentHealth :type "Float (double-precision)"))
  (return (`/Game/Blueprints/BPC_DamageSystem.CurrentHealth` (`self.BPC_DamageSystem`))))

(fn `GetMaxHealth`
  (returns (MaxHealth :type "Float (double-precision)"))
  (return (`/Game/Blueprints/BPC_DamageSystem.MaxHealth` (`self.BPC_DamageSystem`))))

(fn `TakeDamage`
  (params (DamageInfo :type "/Game/Blueprints/S_DamageInfo Structure"))
  (returns (WasDamaged :type Boolean))
  (bind _wasdamaged (`/Game/Blueprints/BPC_DamageSystem.TakeDamage` (`self.BPC_DamageSystem`) DamageInfo))
  (return _wasdamaged))

(fn `UserConstructionScript`
  (bind _bpc_damagesystem (`self.BPC_DamageSystem`))
  (add `/Game/Blueprints/BPC_DamageSystem.OnDeath` _bpc_damagesystem (`|CreateDelegate` :!event `OnDeath`))
  (add `/Game/Blueprints/BPC_DamageSystem.OnDamageResponse` _bpc_damagesystem (`|CreateDelegate` :!event `OnDamageResponse`)))