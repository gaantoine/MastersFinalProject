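; BPC_DamageSystem is a damage component that tracks health and death state for whatever owns it.
; TakeDamage subtracts the incoming DamageInfo amount from CurrentHealth, clamped between zero and MaxHealth, and ignores hits once IsDead is set.
; It fires the OnDeath dispatcher when health runs out, or OnDamageResponse otherwise, leaving reactions to listeners.
; The event graph holds only disabled default events.
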(fn `TakeDamage`
  (params (DamageInfo :type "/Game/Blueprints/S_DamageInfo Structure"))
  (returns (WasDamaged :type Boolean))
  (if (not (`self.IsDead`))
    (bind _output_get (set `self.CurrentHealth` (`KismetMathLibrary.FClamp` (- (`self.CurrentHealth`) (`.DamageAmount_2_8DFFFF574E4A35E1F579F9B682DF55AF` (break `/Game/Blueprints/S_DamageInfo` DamageInfo))) 0.0 (`self.MaxHealth`))))
    (if (<= _output_get 0.0)
      (set `self.IsDead` true)
      (`self.OnDeath`)
      (else
        (`self.OnDamageResponse`)))
    (return true)))