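; Component that edits the actor lists of the level's BP_PuzzleManager at runtime.
; On BeginPlay it caches the manager via GetActorOfClass.
; Add and Remove functions update its puzzle, destination and NPC arrays with AddUnique or checked removal, and ModifyPuzzleManagerLists calls all six in sequence.
; The puzzle actor functions also apply the component's own add and remove arrays alongside the passed-in ones.
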(event `self.ReceiveBeginPlay`
  (bind _returnvalue (`GameplayStatics.GetActorOfClass` "/Game/Blueprints/BP_PuzzleManager.BP_PuzzleManager_C"))
  (set `self.PuzzleManager` _returnvalue))

(fn `AddDestinationActors`
  (params (DestinationsToAdd :type "Array of /Game/Blueprints/BP_TargetDestination Object Reference"))
  (bind _destinationstoadd (`self.DestinationsToAdd`))
  (if (not (`KismetArrayLibrary.Array_IsEmpty` DestinationsToAdd))
    (for _array_element DestinationsToAdd
      (`KismetArrayLibrary.Array_AddUnique` (`/Game/Blueprints/BP_PuzzleManager.DestinationActors` (`self.PuzzleManager`)) _array_element)))
  (if (not (`KismetArrayLibrary.Array_IsEmpty` _destinationstoadd))
    (for _array_element_2 _destinationstoadd
      (`KismetArrayLibrary.Array_AddUnique` (`/Game/Blueprints/BP_PuzzleManager.DestinationActors` (`self.PuzzleManager`)) _array_element_2))
    (return)))

(fn `AddNPCActors`
  (params (NPCsToAdd :type "Array of /Game/AI/BP_NPC Object Reference"))
  (bind _npcstoadd (`self.NPCsToAdd`))
  (if (not (`KismetArrayLibrary.Array_IsEmpty` NPCsToAdd))
    (for _array_element NPCsToAdd
      (`KismetArrayLibrary.Array_AddUnique` (`/Game/Blueprints/BP_PuzzleManager.NPCActors` (`self.PuzzleManager`)) _array_element)))
  (if (not (`KismetArrayLibrary.Array_IsEmpty` _npcstoadd))
    (for _array_element_2 _npcstoadd
      (`KismetArrayLibrary.Array_AddUnique` (`/Game/Blueprints/BP_PuzzleManager.NPCActors` (`self.PuzzleManager`)) _array_element_2))
    (return)))

(fn `AddPuzzleActors`
  (params (ActorsToAdd :type "Array of Actor Object Reference"))
  (bind _puzzleactorstoadd (`self.PuzzleActorsToAdd`))
  (bind _puzzleactors (`/Game/Blueprints/BP_PuzzleManager.PuzzleActors` (`self.PuzzleManager`)))
  (if (not (`KismetArrayLibrary.Array_IsEmpty` ActorsToAdd))
    (for _array_element ActorsToAdd
      (`KismetArrayLibrary.Array_AddUnique` _puzzleactors _array_element)))
  (if (not (`KismetArrayLibrary.Array_IsEmpty` _puzzleactorstoadd))
    (for _array_element_2 _puzzleactorstoadd
      (`KismetArrayLibrary.Array_AddUnique` _puzzleactors _array_element_2))
    (return)))

(fn `ModifyPuzzleManagerLists`
  (params (PuzzleActorsToAdd :type "Array of Actor Object Reference") (PuzzleActorsToRemove :type "Array of Actor Object Reference") (DestinationsToAdd :type "Array of /Game/Blueprints/BP_TargetDestination Object Reference") (DestinationsToRemove :type "Array of /Game/Blueprints/BP_TargetDestination Object Reference") (NPCsToAdd :type "Array of /Game/AI/BP_NPC Object Reference") (NPCsToRemove :type "Array of /Game/AI/BP_NPC Object Reference"))
  (`self.AddPuzzleActors` PuzzleActorsToAdd)
  (`self.RemovePuzzleActors` PuzzleActorsToRemove)
  (`self.AddDestinationActors` DestinationsToAdd)
  (`self.RemoveDestinationActors` DestinationsToRemove)
  (`self.AddNPCActors` NPCsToAdd)
  (`self.RemoveNPCActors` NPCsToRemove)
  (return))

(fn `RemoveDestinationActors`
  (params (DestinationsToRemove :type "Array of /Game/Blueprints/BP_TargetDestination Object Reference"))
  (bind _destinationstoremove (`self.DestinationsToRemove`))
  (bind _destinationactors (`/Game/Blueprints/BP_PuzzleManager.DestinationActors` (`self.PuzzleManager`)))
  (bind _destinationactors_2 (`/Game/Blueprints/BP_PuzzleManager.DestinationActors` (`self.PuzzleManager`)))
  (if (not (`KismetArrayLibrary.Array_IsEmpty` DestinationsToRemove))
    (for _array_element DestinationsToRemove
      (if (`KismetArrayLibrary.Array_Contains` _destinationactors_2 _array_element)
        (`KismetArrayLibrary.Array_RemoveItem` _destinationactors_2 _array_element))))
  (if (not (`KismetArrayLibrary.Array_IsEmpty` _destinationstoremove))
    (for _array_element_2 _destinationstoremove
      (if (`KismetArrayLibrary.Array_Contains` _destinationactors _array_element_2)
        (`KismetArrayLibrary.Array_RemoveItem` _destinationactors _array_element_2)))
    (return)))

(fn `RemoveNPCActors`
  (params (NPCsToRemove :type "Array of /Game/AI/BP_NPC Object Reference"))
  (bind _npcstoremove (`self.NPCsToRemove`))
  (bind _npcactors (`/Game/Blueprints/BP_PuzzleManager.NPCActors` (`self.PuzzleManager`)))
  (bind _npcactors_2 (`/Game/Blueprints/BP_PuzzleManager.NPCActors` (`self.PuzzleManager`)))
  (if (not (`KismetArrayLibrary.Array_IsEmpty` NPCsToRemove))
    (for _array_element NPCsToRemove
      (if (`KismetArrayLibrary.Array_Contains` _npcactors_2 _array_element)
        (`KismetArrayLibrary.Array_RemoveItem` _npcactors_2 _array_element))))
  (if (not (`KismetArrayLibrary.Array_IsEmpty` _npcstoremove))
    (for _array_element_2 _npcstoremove
      (if (`KismetArrayLibrary.Array_Contains` _npcactors _array_element_2)
        (`KismetArrayLibrary.Array_RemoveItem` _npcactors _array_element_2)))
    (return)))

(fn `RemovePuzzleActors`
  (params (ActorsToRemove :type "Array of Actor Object Reference"))
  (bind _puzzleactorstoremove (`self.PuzzleActorsToRemove`))
  (bind _puzzleactors (`/Game/Blueprints/BP_PuzzleManager.PuzzleActors` (`self.PuzzleManager`)))
  (bind _puzzleactors_2 (`/Game/Blueprints/BP_PuzzleManager.PuzzleActors` (`self.PuzzleManager`)))
  (if (not (`KismetArrayLibrary.Array_IsEmpty` ActorsToRemove))
    (for _array_element ActorsToRemove
      (if (`KismetArrayLibrary.Array_Contains` _puzzleactors_2 _array_element)
        (`KismetArrayLibrary.Array_RemoveItem` _puzzleactors_2 _array_element))))
  (if (not (`KismetArrayLibrary.Array_IsEmpty` _puzzleactorstoremove))
    (for _array_element_2 _puzzleactorstoremove
      (if (`KismetArrayLibrary.Array_Contains` _puzzleactors _array_element_2)
        (`KismetArrayLibrary.Array_RemoveItem` _puzzleactors _array_element_2)))
    (return)))