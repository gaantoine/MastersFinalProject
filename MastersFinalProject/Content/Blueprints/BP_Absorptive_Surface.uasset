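; BP_Absorptive_Surface is a surface actor that slides between its start position and an offset, optionally controlled by linked pressure plates.
; The construction script binds to each plate's toggle event, which recounts active plates to allow activation when all are active, or none with ReverseActivation.
; Activation plays a timeline that lerps the root's world location, or reverses it when disallowed.
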(event `self.ReceiveBeginPlay`
  (set `self.StartPosition` (`SceneComponent.K2_GetComponentLocation` (`self.DefaultSceneRoot`))))

(event `PlatesToggled`
  (params (PlateToggled :type "/Game/Blueprints/BP_PressurePlate Object Reference"))
  (if (`self.IsPlateControlled`)
    (set `self.ActivatedPlateCount` 0)
    (for _array_element (`self.LinkedPressurePlates`)
      (if (`/Game/Blueprints/BP_PressurePlate.PlateActive` _array_element)
        (`/Engine/EditorBlueprintResources/StandardMacros.IncrementInt` (`self.ActivatedPlateCount`))))
    (if (`self.ReverseActivation`)
      (if (== (`self.ActivatedPlateCount`) 0)
        (set `self.ActivationAllowed` true)
        (message `/Game/Blueprints/BPI_Player_Activation.PlayerActivated` self null)
        (else
          (set `self.ActivationAllowed` false)
          (message `/Game/Blueprints/BPI_Player_Activation.PlayerActivated` self null)))
      (elif (== (`self.ActivatedPlateCount`) (`KismetArrayLibrary.Array_Length` (`self.LinkedPressurePlates`)))
        (set `self.ActivationAllowed` true)
        (message `/Game/Blueprints/BPI_Player_Activation.PlayerActivated` self null)
        (else
          (set `self.ActivationAllowed` false)
          (message `/Game/Blueprints/BPI_Player_Activation.PlayerActivated` self null))))))

(event `/Game/Blueprints/BPI_Player_Activation.PlayerActivated`
  (params (Player :type "/Game/FirstPerson/Blueprints/BP_FirstPersonCharacter Object Reference"))
  (bind _startposition (`self.StartPosition`))
  (if (`self.ActivationAllowed`)
    (bind (_direction _actorposition) (`Timeline|ActorMovementTimeline` :!label _label)
      (:`Update`
        (`SceneComponent.K2_SetWorldLocation` (`self.DefaultSceneRoot`) (`KismetMathLibrary.VLerp` _startposition (+ _startposition (`self.EndPosition`)) _actorposition) false false)))
    (else
      (goto _label :!via `Reverse`))))

(fn `UserConstructionScript`
  (if (`self.IsPlateControlled`)
    (for _array_element (`self.LinkedPressurePlates`)
      (add `/Game/Blueprints/BP_PressurePlate.PlateToggled` _array_element (`|CreateDelegate` :!event `PlatesToggled`)))))