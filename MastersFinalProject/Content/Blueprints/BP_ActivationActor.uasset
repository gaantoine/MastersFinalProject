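; Puzzle activation actor that reacts to a SoundReceived event, with a configurable static mesh applied in the construction script.
; When flagged to modify the puzzle manager, it updates the manager's lists once through BPCPuzzleManagerModifier, guarded by a DoOnce.
; When flagged as having linked actors, it sends RespondToLinkedActorMessage to each entry in LinkedActors.
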(event `/Game/Blueprints/BPI_Sound_Reaction.SoundReceived`
  (params (Signal :type "/Game/Blueprints/S_Signal Structure"))
  (if (`self.ModifiesPuzzleManager`)
    (`/Engine/EditorBlueprintResources/StandardMacros.DoOnce` false
      (:`Completed`
        (`/Game/Blueprints/BPC_PuzzleManagerModifier.ModifyPuzzleManagerLists` :`self` (`self.BPC_PuzzleManagerModifier`)))))
  (if (`self.HasLinkedActors`)
    (for _array_element (`self.LinkedActors`)
      (message `/Game/Blueprints/BPI_LinkedActor.RespondToLinkedActor` _array_element))))

(fn `UserConstructionScript`
  (`StaticMeshComponent.SetStaticMesh` (`self.StaticMesh`) (`self.StaticMeshToUse`)))