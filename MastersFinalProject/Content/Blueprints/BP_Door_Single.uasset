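; BP_Door_Single is a single door that slides open and closed when it receives an activation signal.
; SoundReceived checks the first three characters of the signal string and calls PlayerActivated on "ACT".
; A FlipFlop alternately plays and reverses the DoorOpen timeline, which lerps the Door's relative location between DoorStart and DoorEnd.
; The ActivationInProgress flag ignores further activations until the timeline finishes.
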(event `/Game/Blueprints/BPI_Sound_Reaction.SoundReceived`
  (params (Signal :type "/Game/Blueprints/S_Signal Structure"))
  (switch `string` (`KismetStringLibrary.GetSubstring` (`.SignalString_2_84FC3C6342EC7A75A318BD98180D617C` (break `/Game/Blueprints/S_Signal` Signal)) 0 3)
    (:`ACT`
      (`/Game/Blueprints/BPI_Player_Activation.PlayerActivated` null))))

(event `/Game/Blueprints/BPI_Player_Activation.PlayerActivated`
  (params (Player :type "/Game/FirstPerson/Blueprints/BP_FirstPersonCharacter Object Reference"))
  (if (not (`self.ActivationInProgress`))
    (set `self.ActivationInProgress` true)
    (`/Engine/EditorBlueprintResources/StandardMacros.FlipFlop`
      (:`A`
        (bind (_direction _doorposition) (`Timeline|DoorOpen` :!label _label)
          (:`Update`
            (`SceneComponent.K2_SetRelativeLocation` (`self.Door`) (`KismetMathLibrary.VLerp` (`self.DoorStart`) (`self.DoorEnd`) _doorposition) false false))
          (:`Finished`
            (set `self.ActivationInProgress` false))))
      (:`B`
        (goto _label :!via `Reverse`)))))

(fn `UserConstructionScript`)