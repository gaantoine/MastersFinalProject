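; Moveable wall actor that slides to an end position, once, when it receives the RespondtoLinkedActor event.
; A timeline drives a lerp of the wall mesh from its current, continually updated relative location toward WallEndPosition.
; The construction script applies a configurable material to the mesh.
; SoundReceived is empty, and the visibility and puzzle manager update nodes are unconnected.
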(event `self.ReceiveBeginPlay`)

(event `self.SoundReceived`
  (params (Signal :type "/Game/Blueprints/S_Signal Structure")))

(event `self.RespondToLinkedActor`
  (`/Engine/EditorBlueprintResources/StandardMacros.DoOnce` false
    (:`Completed`
      (bind (_direction _wallposition) (`Timeline|WallSlideTimeline` :!via `PlayFromStart`)
        (:`Update`
          (`SceneComponent.K2_SetRelativeLocation` (`self.WallMesh`) (`KismetMathLibrary.VLerp` (`SceneComponent.RelativeLocation` (`self.WallMesh`)) (`self.WallEndPosition`) _wallposition) false false))))))

(fn `UserConstructionScript`
  (`PrimitiveComponent.SetMaterial` (`self.WallMesh`) 0 (`self.WallMaterial`)))