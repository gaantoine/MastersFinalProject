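; A door that toggles open and closed when a BP_NPC enters or leaves its construction-sized trigger box, or on an "ACT" sound signal.
; A FlipFlop plays or reverses a timeline that lerps the door's position, ignoring activations mid-move.
; When ModifiesPuzzleManager is set, the first finished move updates puzzle manager lists through a modifier component.
; Events forward list edits to that component, though RemoveDestinations calls its add function.
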(event `self.SoundReceived`
  (params (Signal :type "/Game/Blueprints/S_Signal Structure"))
  (switch `string` (`KismetStringLibrary.GetSubstring` (`.SignalString_2_84FC3C6342EC7A75A318BD98180D617C` (break `/Game/Blueprints/S_Signal` Signal)) 0 3)
    (:`ACT`
      (`/Game/Blueprints/BPI_Player_Activation.PlayerActivated` null))))

(event `self.PlayerActivated`
  (params (Player :type "/Game/FirstPerson/Blueprints/BP_FirstPersonCharacter Object Reference"))
  (if (not (`self.ActivationInProgress`))
    (set `self.ActivationInProgress` true)
    (`/Engine/EditorBlueprintResources/StandardMacros.FlipFlop`
      (:`A`
        (bind (_direction _doorposition) (`Timeline|DoorOpen` :!label _label)
          (:`Update`
            (`SceneComponent.K2_SetRelativeLocation` (`self.Door`) (`KismetMathLibrary.VLerp` (`self.DoorStart`) (`self.DoorEnd`) _doorposition) false false))
          (:`Finished`
            (set `self.ActivationInProgress` false)
            (if (`self.ModifiesPuzzleManager`)
              (`/Engine/EditorBlueprintResources/StandardMacros.DoOnce` false
                (:`Completed`
                  (`KismetSystemLibrary.PrintString` "Modifying Puzzle Manager Lists" true true (struct :`R` 1.0 :`B` 0.885903 :`A` 1.0) 5.0)
                  (`/Game/Blueprints/BPC_PuzzleManagerModifier.ModifyPuzzleManagerLists` :`self` (`self.BPC_PuzzleManagerModifier`))))))))
      (:`B`
        (goto _label :!via `Reverse`)))))

(event `self.AddPuzzleActors`
  (params (ActorsToAdd :type "Array of Actor Object Reference (by ref)"))
  (`/Game/Blueprints/BPC_PuzzleManagerModifier.AddPuzzleActors` (`self.BPC_PuzzleManagerModifier`) ActorsToAdd))

(event `self.RemovePuzzleActors`
  (params (ActorsToRemove :type "Array of Actor Object Reference (by ref)"))
  (`/Game/Blueprints/BPC_PuzzleManagerModifier.RemovePuzzleActors` (`self.BPC_PuzzleManagerModifier`) ActorsToRemove))

(event `self.AddNPCs`
  (params (NPCsToAdd :type "Array of /Game/AI/BP_NPC Object Reference (by ref)"))
  (`/Game/Blueprints/BPC_PuzzleManagerModifier.AddNPCActors` (`self.BPC_PuzzleManagerModifier`) NPCsToAdd))

(event `self.RemoveNPCs`
  (params (NPCsToRemove :type "Array of /Game/AI/BP_NPC Object Reference (by ref)"))
  (`/Game/Blueprints/BPC_PuzzleManagerModifier.RemoveNPCActors` (`self.BPC_PuzzleManagerModifier`) NPCsToRemove))

(event `self.AddDestinations`
  (params (DestinationsToAdd :type "Array of /Game/Blueprints/BP_TargetDestination Object Reference (by ref)"))
  (`/Game/Blueprints/BPC_PuzzleManagerModifier.AddDestinationActors` (`self.BPC_PuzzleManagerModifier`) DestinationsToAdd))

(event `self.RemoveDestinations`
  (params (DestinationsToRemove :type "Array of /Game/Blueprints/BP_TargetDestination Object Reference (by ref)"))
  (`/Game/Blueprints/BPC_PuzzleManagerModifier.AddDestinationActors` (`self.BPC_PuzzleManagerModifier`) DestinationsToRemove))

(event `self.TriggerBox.OnComponentBeginOverlap`
  (params (OverlappedComponent :type "PrimitiveComponent Object Reference") (OtherActor :type "Actor Object Reference") (OtherComp :type "PrimitiveComponent Object Reference") (OtherBodyIndex :type Integer) (bFromSweep :type Boolean) (SweepResult :type "HitResult Structure (by ref)"))
  (cast `/Game/AI/BP_NPC` OtherActor)
  (`/Game/Blueprints/BPI_Player_Activation.PlayerActivated` null))

(event `self.TriggerBox.OnComponentEndOverlap`
  (params (OverlappedComponent :type "PrimitiveComponent Object Reference") (OtherActor :type "Actor Object Reference") (OtherComp :type "PrimitiveComponent Object Reference") (OtherBodyIndex :type Integer))
  (cast `/Game/AI/BP_NPC` OtherActor)
  (`/Game/Blueprints/BPI_Player_Activation.PlayerActivated` null))

(fn `UserConstructionScript`
  (`BoxComponent.SetBoxExtent` (`self.TriggerBox`) (`self.TriggerBoxExtents`) true))