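; BP_PPLockedDoor is a door lock that opens a child BP_Door_Single through linked pressure plates.
; The construction script binds each plate's toggle event and sets the decorator's visibility.
; Each toggle recounts active plates, requiring all active, or none with ReverseActivation.
; Once met, the unlock latches and sends the door its player-activated message once, with debug prints reporting progress.
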(event `self.ReceiveBeginPlay`
  (bind _asbp_door_single (cast `/Game/Blueprints/BP_Door_Single` (`ChildActorComponent.ChildActor` (`self.DoorActor`))))
  (set `self.Door` _asbp_door_single))

(event `PlatesToggled`
  (params (PlateToggled :type "/Game/Blueprints/BP_PressurePlate Object Reference"))
  (bind _activatedplatecount (`self.ActivatedPlateCount`))
  (bind _activatedplatecount_2 (`self.ActivatedPlateCount`))
  (`KismetSystemLibrary.PrintString` (`KismetStringLibrary.Concat_StrStr` "Plate togggled: " (`KismetSystemLibrary.GetDisplayName` PlateToggled)) true true (struct :`R` 0.5 :`B` 1.0 :`A` 1.0) 5.0)
  (if (not (`self.DoorUnlocked`))
    (set `self.ActivatedPlateCount` 0)
    (for _array_element (`self.LinkedPressurePlates`)
      (if (`/Game/Blueprints/BP_PressurePlate.PlateActive` _array_element)
        (`/Engine/EditorBlueprintResources/StandardMacros.IncrementInt` (`self.ActivatedPlateCount`))))
    (if (`self.ReverseActivation`)
      (`KismetSystemLibrary.PrintString` (`KismetStringLibrary.Concat_StrStr` "Plates active: " (`KismetStringLibrary.Conv_IntToString` _activatedplatecount_2)) true true (struct :`R` 0.000428 :`G` 1.0 :`A` 1.0) 5.0)
      (if (== _activatedplatecount_2 0)
        (set `self.DoorUnlocked` true)
        (`KismetSystemLibrary.PrintString` "Door Unlocked" true true (struct :`R` 1.0 :`G` 0.382883 :`A` 1.0) 5.0)
        (`/Engine/EditorBlueprintResources/StandardMacros.DoOnce` false
          (:`Completed`
            (message `/Game/Blueprints/BPI_Player_Activation.PlayerActivated` (`self.Door`) null)))
        (else
          (`KismetSystemLibrary.PrintString` "Reverse activation: Not all plates deactivated.  Door is still locked." true true (struct :`R` 1.0 :`A` 1.0) 5.0)))
      (else
        (`KismetSystemLibrary.PrintString` (`KismetStringLibrary.Concat_StrStr` "Plates active: " (`KismetStringLibrary.Conv_IntToString` _activatedplatecount)) true true (struct :`R` 0.000428 :`G` 1.0 :`A` 1.0) 5.0)
        (if (== _activatedplatecount (`KismetArrayLibrary.Array_Length` (`self.LinkedPressurePlates`)))
          (set `self.DoorUnlocked` true)
          (`KismetSystemLibrary.PrintString` "Door Unlocked" true true (struct :`R` 1.0 :`G` 0.382883 :`A` 1.0) 5.0)
          (`/Engine/EditorBlueprintResources/StandardMacros.DoOnce` false
            (:`Completed`
              (message `/Game/Blueprints/BPI_Player_Activation.PlayerActivated` (`self.Door`) null)))
          (else
            (`KismetSystemLibrary.PrintString` "Not all plates active.  Door is still locked." true true (struct :`R` 1.0 :`A` 1.0) 5.0)))))))

(fn `UserConstructionScript`
  (for _array_element (`self.LinkedPressurePlates`)
    (add `/Game/Blueprints/BP_PressurePlate.PlateToggled` _array_element (`|CreateDelegate` :!event `PlatesToggled`))
    (`SceneComponent.SetVisibility` (`self.Decorator`) (`self.DecoratorVisible`) false)))