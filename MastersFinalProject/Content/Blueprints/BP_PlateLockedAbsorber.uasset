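; Puzzle absorber that slides between two positions depending on the state of its linked pressure plates.
; Plate toggles, bound in the construction script, unlock it when all plates are active, or none with ReverseActivation.
; Activation, also triggerable by "ACT" sound signals, plays or reverses a timeline that moves the Absorber.
; The first timeline finish can update puzzle manager lists through BPCPuzzleManagerModifier; RemoveDestinations calls the component's add function.
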(event `self.SoundReceived`
  (params (Signal :type "/Game/Blueprints/S_Signal Structure"))
  (switch `string` (`KismetStringLibrary.GetSubstring` (`.SignalString_2_84FC3C6342EC7A75A318BD98180D617C` (break `/Game/Blueprints/S_Signal` Signal)) 0 3)
    (:`ACT`
      (if (`self.ShouldRespondToSounds`)
        (`/Game/Blueprints/BPI_Player_Activation.PlayerActivated` null)))))

(event `self.PlayerActivated`
  (params (Player :type "/Game/FirstPerson/Blueprints/BP_FirstPersonCharacter Object Reference"))
  (if (`self.PlatformUnlocked`)
    (bind (_direction _doorposition) (`Timeline|DoorOpen` :!label _label)
      (:`Update`
        (`SceneComponent.K2_SetRelativeLocation` (`self.Absorber`) (`KismetMathLibrary.VLerp` (`self.ReflectorStart`) (`self.ReflectorEnd`) _doorposition) false false))
      (:`Finished`
        (if (`self.ModifiesPuzzleManager`)
          (`/Engine/EditorBlueprintResources/StandardMacros.DoOnce` false
            (:`Completed`
              (`/Game/Blueprints/BPC_PuzzleManagerModifier.ModifyPuzzleManagerLists` :`self` (`self.BPC_PuzzleManagerModifier`)))))))
    (else
      (goto _label :!via `Reverse`))))

(event `self.AddPuzzleActors`
  (params (ActorsToAdd :type "Array of Actor Object Reference (by ref)"))
  (`/Game/Blueprints/BPC_PuzzleManagerModifier.AddPuzzleActors` (`self.BPC_PuzzleManagerModifier`) ActorsToAdd))

(event `self.RemovePuzzleActors`
  (params (ActorsToRemove :type "Array of Actor Object Reference (by ref)"))
  (`/Game/Blueprints/BPC_PuzzleManagerModifier.RemovePuzzleActors` (`self.BPC_PuzzleManagerModifier`) ActorsToRemove))

(event `self.AddNPCs`
  (params (NPCsToAdd :type "Array of /Game/AI/BP_NPC Object Reference (by ref)"))
  (`/Game/Blueprints/BPC_PuzzleManagerModifier.AddNPCActors` (`self.BPC_PuzzleManagerModifier`) NPCsToAdd))

(event `self.RemoveNPCs`
  (params (NPCsToRemove :type "Array of /Game/AI/BP_NPC Object Reference (by ref)"))
  (`/Game/Blueprints/BPC_PuzzleManagerModifier.RemoveNPCActors` (`self.BPC_PuzzleManagerModifier`) NPCsToRemove))

(event `self.AddDestinations`
  (params (DestinationsToAdd :type "Array of /Game/Blueprints/BP_TargetDestination Object Reference (by ref)"))
  (`/Game/Blueprints/BPC_PuzzleManagerModifier.AddDestinationActors` (`self.BPC_PuzzleManagerModifier`) DestinationsToAdd))

(event `self.RemoveDestinations`
  (params (DestinationsToRemove :type "Array of /Game/Blueprints/BP_TargetDestination Object Reference (by ref)"))
  (`/Game/Blueprints/BPC_PuzzleManagerModifier.AddDestinationActors` (`self.BPC_PuzzleManagerModifier`) DestinationsToRemove))

(event `PlatesToggled`
  (params (PlateToggled :type "/Game/Blueprints/BP_PressurePlate Object Reference"))
  (set `self.ActivatedPlateCount` 0)
  (for _array_element (`self.LinkedPressurePlates`)
    (if (`/Game/Blueprints/BP_PressurePlate.PlateActive` _array_element)
      (`/Engine/EditorBlueprintResources/StandardMacros.IncrementInt` (`self.ActivatedPlateCount`))))
  (if (`self.ReverseActivation`)
    (if (== (`self.ActivatedPlateCount`) 0)
      (set `self.PlatformUnlocked` true)
      (message `/Game/Blueprints/BPI_Player_Activation.PlayerActivated` self null)
      (else
        (set `self.PlatformUnlocked` false)
        (message `/Game/Blueprints/BPI_Player_Activation.PlayerActivated` self null)))
    (elif (== (`self.ActivatedPlateCount`) (`KismetArrayLibrary.Array_Length` (`self.LinkedPressurePlates`)))
      (set `self.PlatformUnlocked` true)
      (message `/Game/Blueprints/BPI_Player_Activation.PlayerActivated` self null)
      (else
        (set `self.PlatformUnlocked` false)
        (message `/Game/Blueprints/BPI_Player_Activation.PlayerActivated` self null)))))

(fn `UserConstructionScript`
  (for _array_element (`self.LinkedPressurePlates`)
    (add `/Game/Blueprints/BP_PressurePlate.PlateToggled` _array_element (`|CreateDelegate` :!event `PlatesToggled`))))