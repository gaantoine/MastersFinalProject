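; BP_TutorialGlassWall is a sliding glass wall that displays tutorial text.
; The construction script applies two configurable texts and a shared color to text renderers, which BeginPlay hides.
; SoundReceived reveals them once, waits two seconds, then modifies puzzle manager lists through BPCPuzzleManagerModifier.
; RespondtoLinkedActor plays a one-shot timeline that lerps the mesh from its current world location toward WallEndPosition, setting it as relative location.
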(event `self.ReceiveBeginPlay`
  (`SceneComponent.SetVisibility` (`self.TextRenderer`) false false)
  (`SceneComponent.SetVisibility` (`self.TextRenderer2`) false false))

(event `/Game/Blueprints/BPI_Sound_Reaction.SoundReceived`
  (params (Signal :type "/Game/Blueprints/S_Signal Structure"))
  (`/Engine/EditorBlueprintResources/StandardMacros.DoOnce` false
    (:`Completed`
      (`SceneComponent.SetVisibility` (`self.TextRenderer`) true false)
      (`SceneComponent.SetVisibility` (`self.TextRenderer2`) true false)
      (`KismetSystemLibrary.Delay` 2.0)
      (`/Game/Blueprints/BPC_PuzzleManagerModifier.ModifyPuzzleManagerLists` :`self` (`self.BPC_PuzzleManagerModifier`)))))

(event `/Game/Blueprints/BPI_LinkedActor.RespondToLinkedActor`
  (`/Engine/EditorBlueprintResources/StandardMacros.DoOnce` false
    (:`Completed`
      (bind (_direction _wallposition) (`Timeline|WallSlideTimeline` :!via `PlayFromStart`)
        (:`Update`
          (`SceneComponent.K2_SetRelativeLocation` (`self.GlassWallMesh`) (`KismetMathLibrary.VLerp` (`SceneComponent.K2_GetComponentLocation` (`self.GlassWallMesh`)) (`self.WallEndPosition`) _wallposition) false false))))))

(fn `UserConstructionScript`
  (bind _textrenderer (`self.TextRenderer`))
  (bind _textcolor (`self.TextColor`))
  (bind _textrenderer2 (`self.TextRenderer2`))
  (`TextRenderComponent.K2_SetText` _textrenderer (`self.TutorialText`))
  (`TextRenderComponent.SetTextRenderColor` _textrenderer _textcolor)
  (`TextRenderComponent.K2_SetText` _textrenderer2 (`self.TutorialText2`))
  (`TextRenderComponent.SetTextRenderColor` _textrenderer2 _textcolor))