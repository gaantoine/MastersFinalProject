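; IDTagFront is an actor that displays a four-digit ID number on a TextRender component, as the front side of an ID tag.
; On BeginPlay it builds the number from four random digits and applies the stored FrontIDVisible flag to the text.
; Three update functions let other code set the number, the visibility or both, storing each value and refreshing the text render immediately.
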(event `self.ReceiveBeginPlay`
  (bind _output_get (set `self.IDNumber` (`KismetStringLibrary.Concat_StrStr` (`KismetStringLibrary.Conv_IntToString` (`KismetMathLibrary.RandomIntegerInRange` 0 9)) (`KismetStringLibrary.Conv_IntToString` (`KismetMathLibrary.RandomIntegerInRange` 0 9)) (`KismetStringLibrary.Conv_IntToString` (`KismetMathLibrary.RandomIntegerInRange` 0 9)) (`KismetStringLibrary.Conv_IntToString` (`KismetMathLibrary.RandomIntegerInRange` 0 9)))))
  (`TextRenderComponent.K2_SetText` (`self.TextRender`) (`KismetTextLibrary.Conv_StringToText` _output_get))
  (`SceneComponent.SetVisibility` (`self.TextRender`) (`self.FrontIDVisible`) false))

(fn `UpdateIDTagFront`
  (params (IDNumber :type String) (Visibility :type Boolean))
  (bind _output_get (set `self.IDNumber` IDNumber))
  (`TextRenderComponent.K2_SetText` (`self.TextRender`) (`KismetTextLibrary.Conv_StringToText` _output_get))
  (bind _output_get_2 (set `self.FrontIDVisible` Visibility))
  (`SceneComponent.SetVisibility` (`self.TextRender`) _output_get_2 false))

(fn `UpdateIDTagFrontText`
  (params (IDNumber :type String))
  (bind _output_get (set `self.IDNumber` IDNumber))
  (`TextRenderComponent.K2_SetText` (`self.TextRender`) (`KismetTextLibrary.Conv_StringToText` _output_get)))

(fn `UpdateIDTagFrontVisibility`
  (params (Visibility :type Boolean))
  (bind _output_get (set `self.FrontIDVisible` Visibility))
  (`SceneComponent.SetVisibility` (`self.TextRender`) _output_get false))

(fn `UserConstructionScript`)