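; Trigger-volume actor that plays a one-shot 2D sound when the first-person player looks at a new point of interest.
; Player overlap with the resizable box toggles Tick, which fires randomly deflected camera line traces, approximating a gaze cone, with debug drawing on.
; Hit actors with "POI" in their names are recorded so each triggers once.
; Tick pauses briefly after each find and switches off when the count reaches POIMax.
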(event `self.Trigger.OnComponentBeginOverlap`
  (params (OverlappedComponent :type "PrimitiveComponent Object Reference") (OtherActor :type "Actor Object Reference") (OtherComp :type "PrimitiveComponent Object Reference") (OtherBodyIndex :type Integer) (bFromSweep :type Boolean) (SweepResult :type "HitResult Structure (by ref)"))
  (cast `/Game/FirstPerson/Blueprints/BP_FirstPersonCharacter` OtherActor)
  (`self.SetActorTickEnabled` true))

(event `self.Trigger.OnComponentEndOverlap`
  (params (OverlappedComponent :type "PrimitiveComponent Object Reference") (OtherActor :type "Actor Object Reference") (OtherComp :type "PrimitiveComponent Object Reference") (OtherBodyIndex :type Integer))
  (cast `/Game/FirstPerson/Blueprints/BP_FirstPersonCharacter` OtherActor)
  (`self.SetActorTickEnabled` false))

(event `self.ReceiveTick`
  (params (DeltaSeconds :type "Float (single-precision)"))
  (bind _poilookedat (`self.POILookedAt`))
  (bind _asbp_first_person_character (cast `/Game/FirstPerson/Blueprints/BP_FirstPersonCharacter` (`GameplayStatics.GetPlayerCharacter` 0)))
  (bind _firstpersoncameracomponent (`MastersFinalProjectCharacter.FirstPersonCameraComponent` _asbp_first_person_character))
  (bind _returnvalue (`SceneComponent.K2_GetComponentLocation` _firstpersoncameracomponent))
  (bind _outhit (`KismetSystemLibrary.LineTraceSingle` :`Start` _returnvalue :`End` (+ _returnvalue (* (`KismetMathLibrary.RotateAngleAxis` (`SceneComponent.GetForwardVector` _firstpersoncameracomponent) (`KismetMathLibrary.RandomFloatInRange` 0.0 10.0) (`KismetMathLibrary.MakeVector` 0.0 (`KismetMathLibrary.RandomFloat`) (`KismetMathLibrary.RandomFloat`))) 5000.0)) :`TraceChannel` "TraceTypeQuery1" :`DrawDebugType` "ForDuration"))
  (bind (_bblockinghit _binitialoverlap _time _distance _location _impactpoint _normal _impactnormal _physmat _hitactor) (`GameplayStatics.BreakHitResult` _outhit))
  (if (`KismetStringLibrary.Contains` (`KismetSystemLibrary.GetObjectName` _hitactor) "POI")
    (if (not (`KismetArrayLibrary.Array_Contains` _poilookedat _hitactor))
      (`KismetArrayLibrary.Array_Add` _poilookedat _hitactor)
      (`GameplayStatics.SpawnSound2D` null 1.0 1.0 0.0 null)
      (if (== (`KismetArrayLibrary.Array_Length` _poilookedat) (`self.POIMax`))
        (`self.SetActorTickEnabled` false)
        (else
          (`self.SetActorTickEnabled` false)
          (`KismetSystemLibrary.Delay` 3.0)
          (`self.SetActorTickEnabled` true))))))

(fn `UserConstructionScript`
  (`BoxComponent.SetBoxExtent` (`self.Trigger`) (`self.TriggerExtents`) true))