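; Test actor that shows a random four-digit ID on its TextRender component.
; On BeginPlay it joins four random digits from 0 to 9 into a string, stores it in IDNumber and sets it as the displayed text.
; The overlap, tick and construction graphs are empty, and a duplicate random-ID expression is left unconnected.
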(event `self.ReceiveBeginPlay`
  (bind _output_get (set `self.IDNumber` (`KismetStringLibrary.Concat_StrStr` (`KismetStringLibrary.Conv_IntToString` (`KismetMathLibrary.RandomIntegerInRange` 0 9)) (`KismetStringLibrary.Conv_IntToString` (`KismetMathLibrary.RandomIntegerInRange` 0 9)) (`KismetStringLibrary.Conv_IntToString` (`KismetMathLibrary.RandomIntegerInRange` 0 9)) (`KismetStringLibrary.Conv_IntToString` (`KismetMathLibrary.RandomIntegerInRange` 0 9)))))
  (`TextRenderComponent.K2_SetText` (`self.TextRender`) (`KismetTextLibrary.Conv_StringToText` _output_get)))

(fn `UserConstructionScript`)